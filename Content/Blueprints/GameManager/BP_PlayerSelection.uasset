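; BP_PlayerSelection opens the party-joining menu for a player when play begins.
; After a one-tick delay it caches the BP_PartyManager actor, then calls a server RPC that relays to an owning-client RPC.
; The client event shows the mouse cursor and adds a WG_JoinParty widget to the viewport, passing it the party manager and itself.
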(event Custom|CreateMenuSelectionOnClient
  ;[1 0 0] Run On Owning Client
  (Variables|/Script/Engine.PlayerController|SetbShowMouseCursor (Game|GetPlayerController 0) true)
  (bind _returnvalue (UserInterface|CreateWidget "/Game/Widget/WG_JoinParty.WG_JoinParty_C" 0 (Variables|Default|GetGameRef) self))
  (UserInterface|Viewport|AddtoViewport _returnvalue 0))

(event Custom|CreateMenuSelectionOnServer
  ;[0 1 0] Run On Server
  (CallFunction|CreateMenuSelectiononClient))

(event EventBeginPlay
  (Utilities|FlowControl|DelayUntilNextTick)
  (bind _returnvalue (Actor|GetActorOfClass "/Game/Blueprints/GameManager/BP_PartyManager.BP_PartyManager_C"))
  (Variables|Default|SetGameRef _returnvalue)
  (CallFunction|CreateMenuSelectiononServer))

(fn ConstructionScript)