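; Hunter weapon component that attaches to the arm's GripPoint socket and provides shared shooting logic.
; On BeginPlay it caches the owning BP_Hunter, adds the weapons input mapping context and sets the rifle flag on the first-person AnimBP.
; Shooting runs a debug-drawn camera line trace, damaging only Seekers and test NPCs.
; CheckIfGrabbing releases any physics-handle-held object and reports whether one was held.
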(event EventBeginPlay
  ;[0.2902 0 0.2078] Get Owner + attach
  (bind _asbp_hunter (Utilities|Casting|CastToBP_Hunter (Components|GetOwner)))
  (bind _output_get (Variables|BPWeapon|SetPlayerRef _asbp_hunter))
  (Transformation|AttachComponentToComponent (Variables|/Game/Blueprints/Hunter/BP_Hunter.BP_Hunter_C|GetArm _output_get) "GripPoint" "SnapToTarget" "SnapToTarget" "SnapToTarget" true)
  ;[0.2902 0 0.2078] Add mapping context
  (bind _asplayer_controller (Utilities|Casting|CastToPlayerController (Pawn|GetController (Variables|BPWeapon|GetPlayerRef))))
  (Utilities|IsValid (PlayerController|LocalPlayerSubsystems|GetEnhancedInputLocalPlayerSubsystem _asplayer_controller)
    (:Is%20Valid
      (Input|AddMappingContext (PlayerController|LocalPlayerSubsystems|GetEnhancedInputLocalPlayerSubsystem _asplayer_controller) "/Game/Input/IMC_Weapons.IMC_Weapons" 1 "(bIgnoreAllPressedKeysUntilRelease=True,bForceImmediately=False,bNotifyUserSettings=False)")
      ;[0.2902 0 0.2078] Set up animation
      (bind _asfirst_person_anim_bp (Utilities|Casting|CastToFirstPerson_AnimBP (Components|SkeletalMesh|GetAnimInstance (Variables|/Game/Blueprints/Hunter/BP_Hunter.BP_Hunter_C|GetArm (Variables|BPWeapon|GetPlayerRef)))))
      (Variables|/Game/SkeletalMesh/FirstPersonArms/Animations/FirstPerson_AnimBP.FirstPerson_AnimBP_C|SetHasRifle _asfirst_person_anim_bp true))))

(fn CheckifGrabbing
  (params (PlayerRef :type BP%20Personnage%20Object%20Reference))
  (bind _physicshandle (Variables|/Game/Blueprints/BP_Personnage.BP_Personnage_C|GetPhysicsHandle PlayerRef))
  (Utilities|IsValid (Class|PhysicsHandleComponent|GetGrabbedComponent _physicshandle)
    (:Is%20Valid
      (LocalVariables|SetIsHandle? true)
      (Physics|Components|PhysicsHandle|ReleaseComponent _physicshandle))
    (:Is%20Not%20Valid
      (LocalVariables|SetIsHandle? false)))
  (return (LocalVariables|GetIsHandle?)))

(fn Shooting
  (params (PlayerRef :type BP%20Personnage%20Object%20Reference) (ShootRange :type Float%20%28double-precision%29) (Damage :type Float%20%28double-precision%29))
  (bind _camera (Variables|/Game/Blueprints/BP_Personnage.BP_Personnage_C|GetCamera (Variables|BPWeapon|GetPlayerRef)))
  (bind _returnvalue (Transformation|GetWorldLocation _camera))
  (bind _outhit (Collision|LineTraceByChannel _returnvalue (+ _returnvalue (* (Math|Vector|GetForwardVector _camera) ShootRange)) "TraceTypeQuery1" false 0 "ForDuration"))
  (if (or (Class|GameplayStatics|ObjectIsA (.HitActor (Collision|BreakHitResult _outhit)) "/Game/Blueprints/Seeker/BP_Seeker.BP_Seeker_C") (Class|GameplayStatics|ObjectIsA (.HitActor (Collision|BreakHitResult _outhit)) "/Game/Blueprints/BP_NPCTest.BP_NPCTest_C"))
    (Game|Damage|ApplyDamage (.HitActor (Collision|BreakHitResult _outhit)) Damage 0 PlayerRef)))