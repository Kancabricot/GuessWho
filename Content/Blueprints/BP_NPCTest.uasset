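; BP_NPCTest is a test NPC actor that tracks health (Vie) and destroys itself when it reaches zero.
; Its AnyDamage event subtracts incoming damage, clamps the result between zero and MaxVie, and prints the remaining health.
; When the damage causer is a BP_Hunter, the NPC deals a small fixed amount of damage back to it, even on the killing hit.
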(event Game|Damage|EventAnyDamage
  (params (Damage :type Float%20%28single-precision%29) (DamageType :type Damage%20Type%20Object%20Reference) (InstigatedBy :type Controller%20Object%20Reference) (DamageCauser :type Actor%20Object%20Reference))
  ;[1 1 1] Damage
  (bind _output_get (Variables|Default|SetVie (Math|Float|Clamp(Float) (- (Variables|Default|GetVie) Damage) 0.0 (Variables|Default|GetMaxVie))))
  (Development|PrintString (Utilities|String|ToString(Float) _output_get))
  (if (Class|GameplayStatics|ObjectIsA DamageCauser "/Game/Blueprints/Hunter/BP_Hunter.BP_Hunter_C")
    (Game|Damage|ApplyDamage DamageCauser 1.0 0 0))
  (if (== (Variables|Default|GetVie) 0.0)
    (Actor|DestroyActor)))

(fn ConstructionScript)