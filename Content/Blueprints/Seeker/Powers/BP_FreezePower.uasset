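; BP_FreezePower is a Seeker power that stuns nearby Hunters for a set Duration.
; On the weapon ability input, it runs a multi sphere trace of the given Radius at the player's location, with debug drawing enabled.
; Each hit actor that is a BP_Hunter receives a StuntMaximator call with the Duration.
; A test event triggers the same trace.
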(event Custom|test
  (bind _playerref (Variables|Default|GetPlayerRef))
  (bind _returnvalue (Transformation|GetActorLocation _playerref))
  (bind _outhits (Collision|MultiSphereTraceByChannel _returnvalue _returnvalue (Variables|Default|GetRadius) "TraceTypeQuery1" false 0 "ForDuration"))
  (for _array_element _outhits
    (if (Class|GameplayStatics|ObjectIsA (.HitActor (Collision|BreakHitResult _array_element)) "/Game/Blueprints/Hunter/BP_Hunter.BP_Hunter_C")
      (bind _asbp_hunter (Utilities|Casting|CastToBP_Hunter (.HitActor (Collision|BreakHitResult _array_element))))
      (Default|StuntMaximator _asbp_hunter (Variables|Default|GetDuration)))))

(event Input|EnhancedActionEvents|EnhancedInputActionIA_WeaponAbility
  (params (ActionValue :type Boolean) (ElapsedSeconds :type Float%20%28double-precision%29) (TriggeredSeconds :type Float%20%28double-precision%29) (InputAction :type Input%20Action%20Object%20Reference :default "/Game/Input/Actions/IA_WeaponAbility.IA_WeaponAbility"))
  (bind _playerref (Variables|Default|GetPlayerRef))
  (bind _returnvalue (Transformation|GetActorLocation _playerref))
  (bind _outhits (Collision|MultiSphereTraceByChannel _returnvalue _returnvalue (Variables|Default|GetRadius) "TraceTypeQuery1" false 0 "ForDuration"))
  (for _array_element _outhits
    (if (Class|GameplayStatics|ObjectIsA (.HitActor (Collision|BreakHitResult _array_element)) "/Game/Blueprints/Hunter/BP_Hunter.BP_Hunter_C")
      (bind _asbp_hunter (Utilities|Casting|CastToBP_Hunter (.HitActor (Collision|BreakHitResult _array_element))))
      (Default|StuntMaximator _asbp_hunter (Variables|Default|GetDuration)))))

(event EventBeginPlay
  (|CallParentFunction))