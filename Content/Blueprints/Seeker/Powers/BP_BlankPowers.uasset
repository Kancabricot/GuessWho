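; BP_BlankPowers is a bare Seeker power Blueprint that contains only setup logic and no ability behavior.
; On BeginPlay it casts its owner to BP_Seeker, stores it as PlayerRef, and snaps onto the Seeker's Sphere at the GripPoint socket.
; It then adds the IMC_Weapons Enhanced Input mapping context to the owning player controller's local player subsystem, stopping early if either cast fails.
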(event EventBeginPlay
  ;[0.2902 0 0.2078] Get Owner + attach
  (bind _asbp_seeker (Utilities|Casting|CastToBP_Seeker (Components|GetOwner)))
  (bind _output_get (Variables|Default|SetPlayerRef _asbp_seeker))
  (Transformation|AttachComponentToComponent (Variables|/Game/Blueprints/Seeker/BP_Seeker.BP_Seeker_C|GetSphere _output_get) "GripPoint" "SnapToTarget" "SnapToTarget" "SnapToTarget" true)
  ;[0.2902 0 0.2078] Add mapping context
  (bind _asplayer_controller (Utilities|Casting|CastToPlayerController (Pawn|GetController (Variables|Default|GetPlayerRef))))
  (Utilities|IsValid (PlayerController|LocalPlayerSubsystems|GetEnhancedInputLocalPlayerSubsystem _asplayer_controller)
    (:Is%20Valid
      (Input|AddMappingContext (PlayerController|LocalPlayerSubsystems|GetEnhancedInputLocalPlayerSubsystem _asplayer_controller) "/Game/Input/IMC_Weapons.IMC_Weapons" 1 "(bIgnoreAllPressedKeysUntilRelease=True,bForceImmediately=False,bNotifyUserSettings=False)"))))