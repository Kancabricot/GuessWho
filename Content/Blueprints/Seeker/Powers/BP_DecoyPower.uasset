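; Seeker decoy power that hides the player among randomly chosen NPC actors when the weapon ability input fires.
; It spawns a batch of random NPC classes at random offsets within a radius around the player, keeping the player's height.
; It then moves the player to another random offset and gives their Sphere component a random material from a list.
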(event Input|EnhancedActionEvents|EnhancedInputActionIA_WeaponAbility
  (params (ActionValue :type Boolean) (ElapsedSeconds :type Float%20%28double-precision%29) (TriggeredSeconds :type Float%20%28double-precision%29) (InputAction :type Input%20Action%20Object%20Reference :default "/Game/Input/Actions/IA_WeaponAbility.IA_WeaponAbility"))
  (bind _returnvalue (Math|Random|RandomUnitVector))
  (bind _playerref (Variables|Default|GetPlayerRef))
  (bind _radius (Variables|Default|GetRadius))
  (bind _playerref_2 (Variables|Default|GetPlayerRef))
  (bind _returnvalue_2 (Transformation|GetActorLocation _playerref))
  (bind _returnvalue_3 (Transformation|GetActorLocation _playerref_2))
  (bind _returnvalue_4 (* _returnvalue _radius))
  (bind _returnvalue_5 (+ _returnvalue_2 _returnvalue_4))
  ;[1 1 1] Decoy
  (for _index (range 0 5)
    (Game|SpawnActorfromClass (.OutItem (Utilities|Array|Random (Variables|Default|GetNPC))) (Math|Transform|MakeTransform (Math|Vector|MakeVector (.x _returnvalue_5) (.y _returnvalue_5) (.z _returnvalue_3)) "0, 0, 0" "1.000000,1.000000,1.000000") "Undefined" "MultiplyWithRoot" 0 0))
  (Transformation|SetActorLocation (Variables|Default|GetPlayerRef) (Math|Vector|MakeVector (.x _returnvalue_5) (.y _returnvalue_5) (.z _returnvalue_3)) false false)
  (Rendering|Material|SetMaterial (Variables|/Game/Blueprints/Seeker/BP_Seeker.BP_Seeker_C|GetSphere (Variables|Default|GetPlayerRef)) 0 (.OutItem (Utilities|Array|Random (Variables|Default|GetMaterial)))))

(event EventBeginPlay
  (|CallParentFunction))