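; BP_TeleportPower is a Seeker power that teleports the player toward where the camera looks when the weapon ability input fires.
; It line traces 1000 units forward from the camera on the Visibility channel, with debug drawing left on.
; The player moves to the hit location, or to the trace end when nothing blocks, without sweeping or offsetting from the surface.
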(event Input|EnhancedActionEvents|EnhancedInputActionIA_WeaponAbility
  (params (ActionValue :type Boolean) (ElapsedSeconds :type Float%20%28double-precision%29) (TriggeredSeconds :type Float%20%28double-precision%29) (InputAction :type Input%20Action%20Object%20Reference :default "/Game/Input/Actions/IA_WeaponAbility.IA_WeaponAbility"))
  (bind _playerref (Variables|Default|GetPlayerRef))
  (bind _playerref_2 (Variables|Default|GetPlayerRef))
  (bind _camera (Variables|/Game/Blueprints/BP_Personnage.BP_Personnage_C|GetCamera _playerref))
  (bind _returnvalue (Transformation|GetWorldLocation _camera))
  (bind _outhit (Collision|LineTraceByChannel _returnvalue (+ _returnvalue (* (Math|Vector|GetForwardVector _camera) 1000)) "TraceTypeQuery1" false 0 "ForDuration"))
  (if (.bBlockingHit (Collision|BreakHitResult _outhit))
    (Transformation|SetActorLocation _playerref_2 (.Location (Collision|BreakHitResult _outhit)) false true)
    (else
      (Transformation|SetActorLocation _playerref_2 (.TraceEnd (Collision|BreakHitResult _outhit)) false true))))

(event EventBeginPlay
  (|CallParentFunction))